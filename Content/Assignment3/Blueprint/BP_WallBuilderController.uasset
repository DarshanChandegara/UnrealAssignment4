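; Wall builder controller Blueprint that owns the on-screen widget used to show short notification messages.
; CreateWidget creates and stores the widget, adds it to the viewport and hides its notification text.
; Notify displays a given message in that text, then hides it again after a brief Delay.
; BeginPlay, Tick and the construction script are empty, so both custom events rely on being called.
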(event `self.CreateWidget`
  (bind _returnvalue (`|CreateWidget` "/Game/Assignment3/Blueprint/MyWidget.MyWidget_C"))
  (bind _output_get (set `self.MyWidget` _returnvalue))
  (`UserWidget.AddToViewport` _output_get 0)
  (`Widget.SetVisibility` (`/Game/Assignment3/Blueprint/MyWidget.NotificationText` _output_get) "Hidden"))

(event `self.Notify`
  (params (message :type String))
  (bind _notificationtext (`/Game/Assignment3/Blueprint/MyWidget.NotificationText` (`self.MyWidget`)))
  (`Widget.SetVisibility` _notificationtext "Visible")
  (set `TextBlock.Text` (`KismetTextLibrary.Conv_StringToText` message) _notificationtext)
  (`KismetSystemLibrary.Delay` 2.0)
  (set `Widget.Visibility` "Hidden" _notificationtext))

(fn `UserConstructionScript`)